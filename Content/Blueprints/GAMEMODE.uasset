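; Game mode that tracks the player's friend count, total score and individual score and shows them on a live score HUD.
; On BeginPlay it creates the LiveScore widget, keeps a reference and adds it to the viewport.
; Three update events each add a delta to their stored value, clamp it at zero and write it straight to the widget.
; A Reset event zeroes all three counters and their HUD values.
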(event `Reset`
  (bind _hud (`self.HUD`))
  ;[1 1 1] reset gaame
  (set `/Game/Blueprints/LiveScore.No of f` 0 _hud)
  (set `/Game/Blueprints/LiveScore.Total score` 0 _hud)
  (set `/Game/Blueprints/LiveScore.individual score` 0 _hud)
  (set `self.Current Friends` 0)
  (set `self.Current t score` 0)
  (set `self.current i score` 0))

(event `self.ReceiveBeginPlay`
  ;[1 1 1] reset gaame
  (bind _returnvalue (`|CreateWidget` "/Game/Blueprints/LiveScore.LiveScore_C"))
  (bind _output_get (set `self.HUD` _returnvalue))
  (`UserWidget.AddToViewport` _output_get 0))

(event `UpdateScore t score`
  (params (`Total score` :type Integer))
  (bind _returnvalue (+ `Total score` (`self.Current t score`)))
  ;[1 1 1] Update total score
  (if (<= _returnvalue 0)
    (set `self.Current t score` 0)
    (else
      (set `self.Current t score` _returnvalue)))
  (set `/Game/Blueprints/LiveScore.Total score` (`self.Current t score`) (`self.HUD`)))

(event `UpdateScore i score`
  (params (`individual score` :type Integer))
  (bind _returnvalue (+ `individual score` (`self.current i score`)))
  ;[1 1 1] Update individual score
  (if (<= _returnvalue 0)
    (set `self.current i score` 0)
    (else
      (set `self.current i score` _returnvalue)))
  (set `/Game/Blueprints/LiveScore.individual score` (`self.current i score`) (`self.HUD`)))

(event `UpdateScore friends`
  (params (`No of f` :type Integer))
  (bind _returnvalue (+ `No of f` (`self.Current Friends`)))
  ;[1 1 1] update no. of friends
  (if (<= _returnvalue 0)
    (set `self.Current Friends` 0)
    (else
      (set `self.Current Friends` _returnvalue)))
  (set `/Game/Blueprints/LiveScore.No of f` (`self.Current Friends`) (`self.HUD`)))

(fn `UserConstructionScript`)