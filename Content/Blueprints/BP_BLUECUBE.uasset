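; Blue cube actor that reacts when its Cube component is hit, playing a sound, spawning a non-auto-activated emitter, then destroying itself.
; It spawns a BP_Friends actor at the location and rotation cached on BeginPlay.
; It then updates the GAMEMODE scores: a player pawn hit raises Friends, IScore and TScore, while any other hit lowers Friends and still raises TScore.
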(event `self.Cube.OnComponentHit`
  (params (HitComponent :type "PrimitiveComponent Object Reference") (OtherActor :type "Actor Object Reference") (OtherComp :type "PrimitiveComponent Object Reference") (NormalImpulse :type "Vector Structure") (Hit :type "HitResult Structure (by ref)"))
  (`GameplayStatics.PlaySoundAtLocation` "/Game/Sounds/Cue_Files/blue_Cue.blue_Cue" (`self.Location`) (struct) 1.0 1.0 0.0 null null null)
  (`GameplayStatics.SpawnEmitterAtLocation` "/Game/Blueprints/NewParticleSystem.NewParticleSystem" (`self.Location`) (struct) (1.0 1.0 1.0) true "None" false)
  (`self.K2_DestroyActor`)
  (`|SpawnActorFromClass` "/Game/Blueprints/BP_Friends.BP_Friends_C" (`self.trans form`) "Undefined" "OverrideRootScale" null null)
  (if (== OtherActor (`GameplayStatics.GetPlayerPawn` 0))
    (bind _asgamemode (cast `/Game/Blueprints/GAMEMODE` (`GameplayStatics.GetGameMode`)))
    (`/Game/Blueprints/GAMEMODE.UpdateScore friends` _asgamemode 1)
    (`/Game/Blueprints/GAMEMODE.UpdateScore i score` _asgamemode 10)
    (`/Game/Blueprints/GAMEMODE.UpdateScore t score` _asgamemode 10)
    (else
      (bind _asgamemode_2 (cast `/Game/Blueprints/GAMEMODE` (`GameplayStatics.GetGameMode`)))
      (`/Game/Blueprints/GAMEMODE.UpdateScore friends` _asgamemode_2 -1)
      (`/Game/Blueprints/GAMEMODE.UpdateScore t score` _asgamemode_2 10))))

(event `self.ReceiveBeginPlay`
  (bind _output_get (set `self.Location` (`self.K2_GetActorLocation`)))
  (set `self.trans form` (`KismetMathLibrary.MakeTransform` _output_get (`self.K2_GetActorRotation`))))

(fn `UserConstructionScript`)