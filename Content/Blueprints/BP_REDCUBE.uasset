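; BP_REDCUBE is a penalty cube that costs the player points when hit.
; On a component hit it plays a red cue at its BeginPlay location and reads the total score from the GAMEMODE HUD.
; A zero score pauses the game and shows the LmaoDed widget with the mouse cursor.
; Otherwise it destroys itself and deducts points from both scores through GAMEMODE.
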(event `self.ReceiveBeginPlay`
  (set `self.LOCation` (`self.K2_GetActorLocation`)))

(event `self.Cube.OnComponentHit`
  (params (HitComponent :type "PrimitiveComponent Object Reference") (OtherActor :type "Actor Object Reference") (OtherComp :type "PrimitiveComponent Object Reference") (NormalImpulse :type "Vector Structure") (Hit :type "HitResult Structure (by ref)"))
  (`GameplayStatics.PlaySoundAtLocation` "/Game/Sounds/Cue_Files/red_Cue.red_Cue" (`self.LOCation`) (struct) 1.0 1.0 0.0 null null null)
  (bind _asgamemode (cast `/Game/Blueprints/GAMEMODE` (`GameplayStatics.GetGameMode`)))
  (if (== (`/Game/Blueprints/LiveScore.Total score` (`/Game/Blueprints/GAMEMODE.HUD` _asgamemode)) 0)
    (bind _returnvalue (`|CreateWidget` "/Game/Blueprints/LmaoDed.LmaoDed_C" (`GameplayStatics.GetPlayerController` 0)))
    (`GameplayStatics.SetGamePaused` true)
    (`UserWidget.AddToViewport` _returnvalue 0)
    (set `PlayerController.bShowMouseCursor` true (`GameplayStatics.GetPlayerController` 0))
    (else
      (`self.K2_DestroyActor`)
      (`/Game/Blueprints/GAMEMODE.UpdateScore t score` _asgamemode -10)
      (`/Game/Blueprints/GAMEMODE.UpdateScore i score` _asgamemode -10))))

(fn `UserConstructionScript`)